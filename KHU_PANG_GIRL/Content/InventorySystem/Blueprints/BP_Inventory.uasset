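; Slot-based inventory Blueprint that stores item classes and amounts and shows them in an on-screen widget.
; BeginPlay sizes the slot array and creates WBP_QuestWidget, whose InventoryWidget refreshes individual slots as they change.
; AddItem recursively fills partial stacks, then empty slots, capping stacks at MaxStackSize and placing non-stackable items singly.
; Helper functions find free slots or stacks and read slot contents, using item class defaults for item info.
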(event `self.ReceiveBeginPlay`
  (`KismetArrayLibrary.Array_Resize` (`self.Slots`) (`self.AmountOfSlots`))
  (bind _returnvalue (`|CreateWidget` "/Game/EasyQuests/Widgets/WBP_QuestWidget.WBP_QuestWidget_C" null null self (`self.Slots Per Row`)))
  (bind _output_get (set `self.MainWidget` _returnvalue))
  (set `self.Inventory Widget` (`/Game/EasyQuests/Widgets/WBP_QuestWidget.InventoryWidget` _output_get))
  (`UserWidget.AddToViewport` (`self.MainWidget`) 0))

(event `UpdateSlotAtIndex`
  (params (Index :type Integer))
  (`/Game/InventorySystem/Widgets/InventorySlot.UpdateSlot` (`|GetArrayItem` (`/Game/InventorySystem/Widgets/Inventory.SlotsWidgets` (`self.Inventory Widget`)) Index)))

(fn `AddItem`
  (params (ItemClass :type "/Game/InventorySystem/Blueprints/ItemClasses/BP_MasterItem Class Reference") (Amount :type Integer))
  (returns (Success :type Boolean) (Rest :type Integer))
  (locals (localClass :type "/Game/InventorySystem/Blueprints/ItemClasses/BP_MasterItem Class Reference") (FoundIndex :type Integer) (localAmount :type Integer))
  (bind _returnvalue (+ (`.Amount_5_4A0C44034A9AB79B01E1538ECCCAC047` (break `/Game/InventorySystem/Blueprints/Structures/S_InventorySlot` (`|GetArrayItem` (`self.Slots`) (`local.FoundIndex`)))) (`local.localAmount`)))
  (set `local.localClass` ItemClass)
  (set `local.localAmount` Amount)
  (if (`.CanBeStacked?_18_4367AFC74AA363589BA4C8944711107A` (break `/Game/InventorySystem/Blueprints/Structures/S_ItemInfo` (defaults `Object` ItemClass)))
    (bind (_success_ _index) (`self.SearchFreeStack` (`local.localClass`)))
    (if _success_
      (set `local.FoundIndex` _index)
      (if (> _returnvalue (`self.MaxStackSize`))
        (set `local.localAmount` (- _returnvalue (`self.MaxStackSize`)))
        (`KismetArrayLibrary.Array_Set` (`self.Slots`) (`local.FoundIndex`) (make `/Game/InventorySystem/Blueprints/Structures/S_InventorySlot` (`local.localClass`) (`self.MaxStackSize`)))
        (`self.UpdateSlotAtIndex` (`local.FoundIndex`))
        (bind (_success _rest) (`self.AddItem` (`local.localClass`) (`local.localAmount`)))
        (return true _rest)
        (else
          (`KismetArrayLibrary.Array_Set` (`self.Slots`) (`local.FoundIndex`) (make `/Game/InventorySystem/Blueprints/Structures/S_InventorySlot` (`local.localClass`) _returnvalue))
          (`self.UpdateSlotAtIndex` (`local.FoundIndex`))
          (return true 0)))
      (else
        (bind (_success__2 _index_2) (`self.SearchEmptySlot`))
        (if _success__2
          (bind _output_get (set `local.FoundIndex` _index_2))
          (if (> (`local.localAmount`) (`self.MaxStackSize`))
            (`KismetArrayLibrary.Array_Set` (`self.Slots`) _output_get (make `/Game/InventorySystem/Blueprints/Structures/S_InventorySlot` (`local.localClass`) (`self.MaxStackSize`)))
            (`self.UpdateSlotAtIndex` (`local.FoundIndex`))
            (bind (_success_2 _rest_2) (`self.AddItem` (`local.localClass`) (- (`local.localAmount`) (`self.MaxStackSize`))))
            (return true _rest_2)
            (else
              (`KismetArrayLibrary.Array_Set` (`self.Slots`) (`local.FoundIndex`) (make `/Game/InventorySystem/Blueprints/Structures/S_InventorySlot` (`local.localClass`) (`local.localAmount`)))
              (`self.UpdateSlotAtIndex` (`local.FoundIndex`))
              (return true 0)))
          (else
            (return false (`local.localAmount`))))))
    (else
      ;[1 1 1] Can be Stacked? bool값이 False인경우
      (bind (_success__3 _index_3) (`self.SearchEmptySlot`))
      (if _success__3
        (bind _output_get_2 (set `local.FoundIndex` _index_3))
        (`KismetArrayLibrary.Array_Set` (`self.Slots`) _output_get_2 (make `/Game/InventorySystem/Blueprints/Structures/S_InventorySlot` (`local.localClass`) 1))
        (`self.UpdateSlotAtIndex` (`local.FoundIndex`))
        (if (> (`local.localAmount`) 1)
          (bind (_success_3 _rest_3) (`self.AddItem` (`local.localClass`) (- (`local.localAmount`) 1)))
          (return true _rest_3)
          (else
            (return true 0)))
        (else
          (return false (`local.FoundIndex`)))))))

(fn `GetAmountAtIndex`
  (params (Index :type Integer))
  (returns (Amount :type Integer))
  (return (`.Amount_5_4A0C44034A9AB79B01E1538ECCCAC047` (break `/Game/InventorySystem/Blueprints/Structures/S_InventorySlot` (`|GetArrayItem` (`self.Slots`) Index)))))

(fn `GetItemInfoAtIndex`
  (params (Index :type Integer))
  (returns (`EmptySlot?` :type Boolean) (ItemInfo :type "/Game/InventorySystem/Blueprints/Structures/S_ItemInfo Structure") (Amount :type Integer))
  (bind (_itemclass _amount) (break `/Game/InventorySystem/Blueprints/Structures/S_InventorySlot` (`|GetArrayItem` (`self.Slots`) Index)))
  ;[1 1 1] Slot 배열에 ItemInfo 인덱스가 존재하면 Empty Slot bool값 false 반환/ 없으면 true 반환하는 함수
  (if (`KismetSystemLibrary.IsValidClass` _itemclass)
    (return false (defaults `Object` _itemclass) _amount)
    (else
      (return true (struct) 0))))

(fn `IsSlotEmpty?`
  (params (Index :type Integer))
  (returns (`Empty?` :type Boolean))
  (return (not (`KismetSystemLibrary.IsValidClass` (`.ItemClass_2_DF3857474B0A4D2326228095B8FBF507` (break `/Game/InventorySystem/Blueprints/Structures/S_InventorySlot` (`|GetArrayItem` (`self.Slots`) Index)))))))

(fn `SearchEmptySlot`
  (returns (`Success?` :type Boolean) (Index :type Integer))
  (locals (localBool :type Boolean) (localIndex :type Integer))
  ;[1 1 1] 비어있는 슬롯을 탐색하는 함수. slot배열을 반복문으로 IsValidClass가 false값을 가지면 LocalBool, LocalIndex를 설정하고 반복문을 멈추고 로컬값들을 반환함.
  (for (_array_element _array_index) (`self.Slots`)
    (if (not (`KismetSystemLibrary.IsValidClass` (`.ItemClass_2_DF3857474B0A4D2326228095B8FBF507` (break `/Game/InventorySystem/Blueprints/Structures/S_InventorySlot` _array_element))))
      (set `local.localBool` true)
      (set `local.localIndex` _array_index)
      (break)))
  (return (`local.localBool`) (`local.localIndex`)))

(fn `SearchFreeStack`
  (params (ItemClass :type "/Game/InventorySystem/Blueprints/ItemClasses/BP_MasterItem Class Reference"))
  (returns (`Success?` :type Boolean) (Index :type Integer))
  (locals (localBool :type Boolean) (localIndex :type Integer))
  ;[1 1 1] stack이 free한지 탐색하는 함수. slot배열을 반복문으로 IsValidClass(클래스가 사용가능한 경우)가 true값을 가지고, MaxStackSize보다 작다면, LocalBool, LocalIndex를 설정하고 반복문을 멈추고 로컬값들을 반환함.
  (for (_array_element _array_index) (`self.Slots`)
    (bind (_itemclass _amount) (break `/Game/InventorySystem/Blueprints/Structures/S_InventorySlot` _array_element))
    (if (`KismetSystemLibrary.IsValidClass` _itemclass)
      (if (and (== _itemclass ItemClass) (< _amount (`self.MaxStackSize`)))
        (set `local.localBool` true)
        (set `local.localIndex` _array_index)
        (break))))
  (return (`local.localBool`) (`local.localIndex`)))

(fn `UserConstructionScript`)