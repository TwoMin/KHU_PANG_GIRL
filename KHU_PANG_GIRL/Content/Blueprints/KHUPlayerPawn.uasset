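; Player character with camera-relative movement, Shift sprint, and a minutes/seconds countdown that pauses the game with a Game_over widget at zero.
; BeginPlay toggles the quest log and spawns a BP_Inventory linked to the player.
; Pressing E sphere-traces forward and sends OnInteractMessage to the hit actor.
; Quest-facing events manage gold, experience with scaling level thresholds, saving through the quest component, and mouse-cursor/input-mode toggling.
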(event `self.ReceiveTick`
  (params (DeltaSeconds :type "Float (single-precision)"))
  ;[1 1 1] TimerCountdown 이벤트
  (`KismetSystemLibrary.Delay` 1.0)
  (if (== (`self.Seconds`) 0)
    (if (== (`self.Minutes`) 0)
      (bind _returnvalue (`|CreateWidget` "/Game/Blueprints/Game_over.Game_over_C"))
      (`UserWidget.AddToViewport` _returnvalue 0)
      (set `PlayerController.bShowMouseCursor` true (`GameplayStatics.GetPlayerController` 0))
      (`GameplayStatics.SetGamePaused` true)
      (else
        (set `self.Seconds` 59)
        (set `self.Minutes` (- (`self.Minutes`) 1))))
    (else
      (set `self.Seconds` (- (`self.Seconds`) 1)))))

(event `Key|E`
  (params (Key :type "Key Structure"))
  (bind _returnvalue (`self.K2_GetActorLocation`))
  (:`Pressed`
    (bind (_outhit _returnvalue_2) (`KismetSystemLibrary.SphereTraceSingleForObjects` _returnvalue (+ _returnvalue (* (`SceneComponent.GetForwardVector` (`self.CapsuleComponent`)) (`self.InteractionRange`))) 50.0 (`|MakeArray` "ObjectTypeQuery2" "ObjectTypeQuery3" :!type "EObjectTypeQuery Enum") false (`|MakeArray` self :!type "Actor Object Reference")))
    (if _returnvalue_2
      (message `/Game/EasyQuests/Blueprints/BPI/BP_BPI_QuestsInteraction.OnInteract` (`.HitActor` (`GameplayStatics.BreakHitResult` _outhit)) self))))

(event `/Game/EasyQuests/Blueprints/BPI/BP_BPI_Quests.ToggleMouseInput`
  (`self.MouseInput`))

(event `AddExperience`
  (params (Amount :type "Float (double-precision)"))
  (bind _output_get (set `self.Experience` (+ (`self.Experience`) Amount)))
  (while (>= _output_get (`self.NeededExperience`))
    (`/Engine/EditorBlueprintResources/StandardMacros.IncrementInt` (`self.Level`)
      (:`  `
        (set `self.NeededExperience` (* (`self.NeededExperience`) 1.5))))))

(event `AddGold`
  (params (Amount :type Integer))
  (set `self.Gold` (+ (`self.Gold`) Amount)))

(event `/Game/EasyQuests/Blueprints/BPI/BP_BPI_Quests.ModifyGold`
  (params (Amount :type Integer))
  (`self.AddGold` Amount))

(event `/Game/EasyQuests/Blueprints/BPI/BP_BPI_Quests.ModifyExperience`
  (params (Amount :type "Float (single-precision)"))
  (`self.AddExperience` Amount))

(event `SaveEXPGold`
  (`/Game/EasyQuests/Blueprints/BP_BPC_PlayerQuestComponent.SaveQuests` (`self.BP_BPC_PlayerQuestComponent`)))

(event `/Game/EasyQuests/Blueprints/BPI/BP_BPI_Quests.LoadExpGoldInfo`
  (params (Level :type Integer) (Gold :type Integer) (Experience :type "Float (single-precision)") (NeededExperience :type "Float (single-precision)"))
  (set `self.Level` Level)
  (set `self.Gold` Gold)
  (set `self.Experience` Experience)
  (set `self.NeededExperience` NeededExperience))

(event `self.ReceiveBeginPlay`
  ;[1 1 1] 인벤토리 및 스마트폰 UI 고정
  (`/Game/EasyQuests/Blueprints/BP_BPC_PlayerQuestComponent.Toggle Quest Log Visibility` (`self.BP_BPC_PlayerQuestComponent`))
  (bind _returnvalue (`|SpawnActorFromClass` "/Game/InventorySystem/Blueprints/BP_Inventory.BP_Inventory_C" (`KismetMathLibrary.MakeTransform` (0.0 0.0 0.0)) "AlwaysSpawn" "OverrideRootScale" null 20 self 4 null))
  (set `self.Inventory Ref` _returnvalue)
  (if (`HeadMountedDisplayFunctionLibrary.IsHeadMountedDisplayEnabled`)
    (`ActorComponent.Activate` (`self.Camera`) false)
    (else
      (`ActorComponent.Activate` (`self.Camera`) false))))

(event `InputAxis|LookUpDown`
  (params (AxisValue :type "Float (single-precision)"))
  ;[1 1 1] 플레이어 이동 및 카메라 회전
  (`self.AddControllerPitchInput` AxisValue))

(event `InputAxis|MoveForBack`
  (params (AxisValue :type "Float (single-precision)"))
  ;[1 1 1] 플레이어 이동 및 카메라 회전
  (`self.AddMovementInput` (`SceneComponent.GetForwardVector` (`self.Camera`)) AxisValue) ; 앞뒤로 이동
)

(event `InputAxis|LookRightLeft`
  (params (AxisValue :type "Float (single-precision)"))
  ;[1 1 1] 플레이어 이동 및 카메라 회전
  (`self.AddControllerYawInput` AxisValue))

(event `InputAxis|MoveRightLeft`
  (params (AxisValue :type "Float (single-precision)"))
  ;[1 1 1] 플레이어 이동 및 카메라 회전
  (`self.AddMovementInput` (`SceneComponent.GetRightVector` (`self.Camera`)) AxisValue) ; 좌우로 이동
)

(event `InputAction|Shift`
  (params (Key :type "Key Structure"))
  (bind _charactermovement (`self.CharacterMovement`))
  ;[1 1 1] 플레이어 이동 및 카메라 회전
  (:`Pressed`
    (set `CharacterMovementComponent.MaxWalkSpeed` 1000.0 _charactermovement) ; 키를 누르면 속도 증가
  )
  (:`Released`
    (set `CharacterMovementComponent.MaxWalkSpeed` 500.0 _charactermovement) ; 키를 때면 속도 복귀
  ))

(fn `GetExperience`
  (returns (Experience :type "Float (double-precision)"))
  (return (`self.Experience`)))

(fn `GetGold`
  (returns (TotalGold :type Integer))
  (return (`self.Gold`)))

(fn `GetLevel`
  (returns (Level :type Integer))
  (return (`self.Level`)))

(fn `GetNeededExperience`
  (returns (NeededExperience :type "Float (double-precision)"))
  (return (`self.NeededExperience`)))

(fn `MouseInput`
  (bind _returnvalue (`GameplayStatics.GetPlayerController` 0))
  (if (`self.MouseVisibility`)
    (set `PlayerController.bShowMouseCursor` false _returnvalue)
    (`WidgetBlueprintLibrary.SetInputMode_GameOnly` _returnvalue)
    (set `self.MouseVisibility` false)
    (else
      (set `PlayerController.bShowMouseCursor` true _returnvalue)
      (`WidgetBlueprintLibrary.SetInputMode_GameAndUIEx` _returnvalue null)
      (set `self.MouseVisibility` true))))

(fn `UserConstructionScript`)